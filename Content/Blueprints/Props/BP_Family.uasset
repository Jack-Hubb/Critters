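; BP_Family is an interactable prop that requests the family screen through the game instance when the nearby player presses interact.
; A sphere overlap tracks whether the player, fetched via GetPlayerMessage at BeginPlay, is in range.
; Tick polls the player's Interacting state and sets OpenFamily on BP_GameInstance unless CreditsOpen is set.
; A pair of DoOnce nodes shows and hides the HUD interact text once per range change.
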(event `self.ReceiveBeginPlay`
  ;[1 1 1] Being play
  (`self.Refresh Player`)
  (bind _playercharacter (message `/Game/Blueprints/Interfaces/BPI_Player.getPlayer` (`self.Player`)))
  (set `self.playerMainRef` _playercharacter))

(event `Refresh Player`
  ;[1 1 1] Refreshs the player into a variable (might not be needed, can test without)
  (bind _playercharacter (message `/Game/Blueprints/Interfaces/BPI_Player.getPlayer` (`GameplayStatics.GetPlayerCharacter` 0)))
  (set `self.Player` _playercharacter))

(event `checkIfOpenCredits`
  ;[1 1 1] Checks if player is in radius and presses interact
  (if (`self.playerInRadius`)
    (if (`/Game/Blueprints/Player/BP_PlayerCharacterParent.interacting` (`self.Player`))
      ;[1 1 1] credits can be opened so give the correct variables to open shop ("openCredits" = true)
      (bind _asbp_game_instance (cast `/Game/Blueprints/Game/BP_GameInstance` (`GameplayStatics.GetGameInstance`)))
      (if (not (`/Game/Blueprints/Game/BP_GameInstance.creditsOpen` _asbp_game_instance))
        (set `/Game/Blueprints/Game/BP_GameInstance.openFamily` true _asbp_game_instance)))))

(event `self.Sphere.OnComponentBeginOverlap`
  (params (OverlappedComponent :type "PrimitiveComponent Object Reference") (OtherActor :type "Actor Object Reference") (OtherComp :type "PrimitiveComponent Object Reference") (OtherBodyIndex :type Integer) (bFromSweep :type Boolean) (SweepResult :type "HitResult Structure (by ref)"))
  ;[1 1 1] Checks if player is in radius
  (if (== OtherActor (`self.Player`))
    (set `self.playerInRadius` true)))

(event `self.ReceiveTick`
  (params (DeltaSeconds :type "Float (single-precision)"))
  (bind _hud (`/Game/Blueprints/Player/BP_MainPlayerCharacter.hud` (`self.playerMainRef`)))
  (`self.checkIfOpenCredits`)
  (if (`self.playerInRadius`)
    (`/Engine/EditorBlueprintResources/StandardMacros.DoOnce` false :!label _label
      (:`Completed`
        (`/Game/Blueprints/Widgets/WBP_Hud.RevealInteractText` _hud)
        (goto _label_2 :!via `Reset`)))
    (else
      (`/Engine/EditorBlueprintResources/StandardMacros.DoOnce` true :!label _label_2
        (:`Completed`
          (`/Game/Blueprints/Widgets/WBP_Hud.HideInteractText` _hud)
          (goto _label :!via `Reset`))))))

(event `self.Sphere.OnComponentEndOverlap`
  (params (OverlappedComponent :type "PrimitiveComponent Object Reference") (OtherActor :type "Actor Object Reference") (OtherComp :type "PrimitiveComponent Object Reference") (OtherBodyIndex :type Integer))
  ;[1 1 1] Checks if player is in radius
  (if (== (`self.Player`) OtherActor)
    (set `self.playerInRadius` false)))

(fn `foodPickup`
  (params (IAvariable :type "Boolean (by ref)"))
  (returns (isPickingUp :type Boolean))
  (return false))

(fn `getAnimOwner`
  (returns (owningCharacter :type "/Game/Blueprints/Player/BP_PlayerCharacterParent Object Reference"))
  (return null))

(fn `getPlayer`
  (returns (PlayerCharacter :type "/Game/Blueprints/Player/BP_MainPlayerCharacter Object Reference"))
  (return null))

(fn `UserConstructionScript`)