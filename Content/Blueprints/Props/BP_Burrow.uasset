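; Burrow prop that serves as a level exit, banking the food collected in the run and returning to the hub.
; The first overlap on its entrance collision messages the overlapping actor to zoom in the HUD exit widget and stun the player.
; After short delays it plays the burrow sound at the saved SFX volume, adds held food to the GameInstance total and opens L_Hub.
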(event `self.ReceiveBeginPlay`
  (bind _asbp_game_instance (cast `/Game/Blueprints/Game/BP_GameInstance` (`GameplayStatics.GetGameInstance`))))

(event `self.BurrowEntrance_Collision.OnComponentBeginOverlap`
  (params (OverlappedComponent :type "PrimitiveComponent Object Reference") (OtherActor :type "Actor Object Reference") (OtherComp :type "PrimitiveComponent Object Reference") (OtherBodyIndex :type Integer) (bFromSweep :type Boolean) (SweepResult :type "HitResult Structure (by ref)"))
  (`/Engine/EditorBlueprintResources/StandardMacros.DoOnce` false
    (:`Completed`
      (bind _playercharacter (message `/Game/Blueprints/Interfaces/BPI_Player.getPlayer` OtherActor))
      (`/Game/Blueprints/Widgets/WBP_Exit.ZoomIn` (`/Game/Blueprints/Widgets/WBP_Hud.WBP_Exit` (`/Game/Blueprints/Player/BP_MainPlayerCharacter.hud` _playercharacter)))
      (message `/Game/Blueprints/Interfaces/BPI_Player.stunnPlayer` _playercharacter)
      (`KismetSystemLibrary.Delay` 2.0)
      (`GameplayStatics.PlaySound2D` "/Game/Audio/SFX/SC_Burrow.SC_Burrow" (`/Game/Blueprints/Game/BP_GameInstance.SFX volume` (stale `self.ReceiveBeginPlay` _asbp_game_instance)) 1.0 0.0 null null)
      (`KismetSystemLibrary.Delay` 1.0)
      (set `/Game/Blueprints/Game/BP_GameInstance.Food` (+ (`/Game/Blueprints/Game/BP_GameInstance.foodHeldInGame` (stale `self.ReceiveBeginPlay` _asbp_game_instance)) (`/Game/Blueprints/Game/BP_GameInstance.Food` (stale `self.ReceiveBeginPlay` _asbp_game_instance))) (stale `self.ReceiveBeginPlay` _asbp_game_instance))
      (`GameplayStatics.OpenLevel` "L_Hub"))))

(fn `UserConstructionScript`)