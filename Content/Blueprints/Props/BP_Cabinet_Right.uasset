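; BP_Cabinet_Right is a cabinet prop that fills itself with random food items when play begins.
; On BeginPlay it gathers six arrow components as spawn points and spawns a random class from its FoodItems array at each arrow's world location and rotation.
; The overlap and tick events are disabled, and the construction script is empty.
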(event `self.ReceiveBeginPlay`
  (bind _output_get (set `self.SpawnLocations` (`|MakeArray` (`self.Arrow`) (`self.Arrow1`) (`self.Arrow2`) (`self.Arrow3`) (`self.Arrow4`) (`self.Arrow5`))))
  (for _array_element _output_get
    (bind (_returnvalue_location _returnvalue_rotation) (`KismetMathLibrary.BreakTransform` (`SceneComponent.K2_GetComponentToWorld` _array_element)))
    (`|SpawnActorFromClass` (`KismetArrayLibrary.Array_Random` (`self.FoodItems`)) (`KismetMathLibrary.MakeTransform` _returnvalue_location _returnvalue_rotation) "Undefined" "MultiplyWithRoot" null null)))

(fn `UserConstructionScript`)