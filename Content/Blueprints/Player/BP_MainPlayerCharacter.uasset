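; Main player character Blueprint that handles health, trap effects, food inventory and the equipped character mesh, returning to the hub level at zero health.
; BeginPlay adds a claw component and sets the mesh from the GameInstance selection, rerun from Tick while its change flag is set.
; Glue slows movement, while cages stop it until Interact mashing outpaces per-tick decay.
; Pickups update inventory and HUD, and Attack overlaps track nearby bugs.
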(event `self.ReceiveBeginPlay`
  (`parent.ReceiveBeginPlay`)
  (bind _asbp_game_instance (cast `/Game/Blueprints/Game/BP_GameInstance` (`GameplayStatics.GetGameInstance`)))
  (`AddComponent|NODE_AddBPC_Claw-0` :`owner` self :!label _label)
  (`SkeletalMeshComponent.SetSkeletalMeshAsset` (`self.Mesh`) (`|GetArrayItem` (`self.Array`) (`/Game/Blueprints/Game/BP_GameInstance.currentlyEquippedCharacter` _asbp_game_instance))))

(event `RefreshPlayer`
  (goto _label))

(event `self.ReceiveTick`
  (params (DeltaSeconds :type "Float (single-precision)"))
  (`parent.ReceiveTick` DeltaSeconds)
  (if (`/Game/Blueprints/Game/BP_GameInstance.changeCharacter` (stale `self.ReceiveBeginPlay` _asbp_game_instance))
    (`self.RefreshPlayer`))
  (if (<= (`self.health`) 0.0)
    (`GameplayStatics.OpenLevelBySoftObjectPtr` "/Game/Maps/L_Hub.L_Hub")
    (else
      (set `self.Playerlocation` (`self.K2_GetActorLocation`))
      (set `self.currPressProgress` (- (`self.currPressProgress`) 10.0))
      (if (`self.isTrapped`)
        (if (>= (`self.currPressProgress`) 9000.0)
          (set `CharacterMovementComponent.MaxWalkSpeed` 600.0 (`self.CharacterMovement`))
          (set `self.isTrapped` false)
          (set `self.currPressProgress` 0.0))))))

(event `/Game/Blueprints/Interfaces/BPI_Player.slowPlayer`
  (params (OnGlue :type Boolean))
  (bind _charactermovement (`self.CharacterMovement`))
  ;[1 1 1] Glue Trap Slowing
  (if OnGlue
    (set `CharacterMovementComponent.MaxWalkSpeed` 100.0 _charactermovement)
    (else
      (set `CharacterMovementComponent.MaxWalkSpeed` 600.0 _charactermovement))))

(event `/Game/Blueprints/Interfaces/BPI_Player.stunnPlayer`
  ;[1 1 1] Cage Trap Stop
  (set `CharacterMovementComponent.MaxWalkSpeed` 0.0 (`self.CharacterMovement`))
  (set `self.isTrapped` true)
  (set `self.currPressProgress` 0.0))

(event `EnhancedInput|/Game/Blueprints/Game/Input/Actions/IA_Interact`
  (params (ActionValue :type Boolean) (ElapsedSeconds :type "Float (double-precision)") (TriggeredSeconds :type "Float (double-precision)") (InputAction :type "InputAction Object Reference" :default "/Game/Blueprints/Game/Input/Actions/IA_Interact.IA_Interact"))
  ;[1 1 1] stun Mash
  (:`Triggered`
    (set `self.interacting` true)
    (if (`self.isTrapped`)
      (set `self.currPressProgress` (+ (`self.currPressProgress`) 200.0)))))

(event `/Game/Blueprints/Interfaces/BPI_Player.addItemToInv`
  (params (Type :type Integer) (Amount :type Integer))
  (bind _inv (`self.Inv`))
  (`KismetArrayLibrary.Array_Set` _inv Type (+ (`|GetArrayItem` _inv Type) Amount))
  (for _ _inv
    _)
  (`/Game/Blueprints/Widgets/WBP_Hud.AddItems` (`self.hud`) Type Amount)
  (`GameplayStatics.PlaySound2D` "/Game/Audio/SFX/SC_Grab.SC_Grab" (`/Game/Blueprints/Game/BP_GameInstance.SFX volume` (stale `self.ReceiveBeginPlay` _asbp_game_instance)) 1.0 0.0 null null))

(event `/Game/Blueprints/Interfaces/BPI_Player.setHudReference`
  (params (hud :type "/Game/Blueprints/Widgets/WBP_Hud Object Reference"))
  (set `self.hud` hud))

(event `self.ReceiveAnyDamage`
  (params (Damage :type "Float (single-precision)") (DamageType :type "DamageType Object Reference") (InstigatedBy :type "Controller Object Reference") (DamageCauser :type "Actor Object Reference"))
  (set `self.health` (- (`self.health`) Damage))
  (`GameplayStatics.PlaySound2D` "/Game/Audio/SFX/SC_Hurt.SC_Hurt" (`/Game/Blueprints/Game/BP_GameInstance.SFX volume` (stale `self.ReceiveBeginPlay` _asbp_game_instance)) 1.0 0.0 null null))

(event `self.Attack.OnComponentBeginOverlap`
  (params (OverlappedComponent :type "PrimitiveComponent Object Reference") (OtherActor :type "Actor Object Reference") (OtherComp :type "PrimitiveComponent Object Reference") (OtherBodyIndex :type Integer) (bFromSweep :type Boolean) (SweepResult :type "HitResult Structure (by ref)"))
  (if (== OtherActor "/Game/Blueprints/Enemies/BP_Bugs.BP_Bugs")
    (`KismetArrayLibrary.Array_Add` (`self.enemyArray`) OtherActor)))

(event `self.Attack.OnComponentEndOverlap`
  (params (OverlappedComponent :type "PrimitiveComponent Object Reference") (OtherActor :type "Actor Object Reference") (OtherComp :type "PrimitiveComponent Object Reference") (OtherBodyIndex :type Integer))
  (if (== OtherActor "/Game/Blueprints/Enemies/BP_Bugs.BP_Bugs")
    (for _array_element (`self.enemyArray`)
      (if (== _array_element OtherActor)
        (`KismetArrayLibrary.Array_RemoveItem` (`self.enemyArray`) _array_element)))))

(fn `foodPickup`
  (params (IAvariable :type "Boolean (by ref)"))
  (returns (isPickingUp :type Boolean))
  (return IAvariable))

(fn `getAnimOwner`
  (returns (owningCharacter :type "/Game/Blueprints/Player/BP_PlayerCharacterParent Object Reference"))
  (return self))

(fn `getPlayer`
  (returns (PlayerCharacter :type "/Game/Blueprints/Player/BP_MainPlayerCharacter Object Reference"))
  (return self))

(fn `getShop`
  (returns (Shop :type "/Game/Blueprints/Props/BP_Shop Object Reference"))
  (return null))

(fn `UserConstructionScript`
  (`parent.UserConstructionScript`))