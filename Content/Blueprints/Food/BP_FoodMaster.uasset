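; BP_FoodMaster is a food actor, apparently a base class, that slides toward the player character during interaction.
; While IA_Interact is held, plus 0.2 seconds after release, Tick pulls it toward player 0 if within 150 units.
; The pull applies a normalized world-space direction, scaled by Speed and delta time, as a local offset without sweep.
; StunnPlayer only sets PlayStunned, and the pickup and getter functions are empty stubs.
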(event `self.ReceiveBeginPlay`)

(event `EnhancedInput|/Game/Blueprints/Game/Input/Actions/IA_Interact`
  (params (ActionValue :type Boolean) (ElapsedSeconds :type "Float (double-precision)") (TriggeredSeconds :type "Float (double-precision)") (InputAction :type "InputAction Object Reference" :default "/Game/Blueprints/Game/Input/Actions/IA_Interact.IA_Interact"))
  (:`Triggered`
    (set `self.PickingUp` true))
  (:`Completed`
    (`KismetSystemLibrary.Delay` 0.2)
    (set `self.PickingUp` false)))

(event `self.ReceiveTick`
  (params (DeltaSeconds :type "Float (single-precision)"))
  (set `self.Target` (`GameplayStatics.GetPlayerCharacter` 0))
  (if (and (`self.PickingUp`) (<= (`KismetMathLibrary.Vector_Distance` (`self.K2_GetActorLocation` self) (`self.K2_GetActorLocation` (`GameplayStatics.GetPlayerCharacter` 0))) 150.0))
    (`self.PullTowardsTarget`)))

(event `PullTowardsTarget`
  (`self.K2_AddActorLocalOffset` self (* (`KismetMathLibrary.Normal` (- (`self.K2_GetActorLocation` (`self.Target`)) (`self.K2_GetActorLocation`))) (`GameplayStatics.GetWorldDeltaSeconds`) (`self.Speed`)) false false))

(event `/Game/Blueprints/Interfaces/BPI_Player.stunnPlayer`
  (set `self.playStunned` true))

(fn `foodPickup`
  (params (IAvariable :type "Boolean (by ref)"))
  (returns (isPickingUp :type Boolean))
  (return false))

(fn `getAnimOwner`
  (returns (owningCharacter :type "/Game/Blueprints/Player/BP_PlayerCharacterParent Object Reference"))
  (return null))

(fn `getPlayer`
  (returns (PlayerCharacter :type "/Game/Blueprints/Player/BP_MainPlayerCharacter Object Reference"))
  (return null))

(fn `UserConstructionScript`)