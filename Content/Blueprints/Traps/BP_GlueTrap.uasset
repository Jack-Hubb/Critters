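; BP_GlueTrap is a trap actor that slows the player while they stand inside its Box collision.
; Box overlap begin and end send SlowPlayerMessage on and off, ignoring anything other than player character 0.
; Entry also creates and plays a 2D glue sound at the GameInstance's SFX volume, and exit stops it.
; FoodPickup, GetAnimOwner and GetPlayer are empty stubs.
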(event `self.ReceiveBeginPlay`
  (bind _asbp_game_instance (cast `/Game/Blueprints/Game/BP_GameInstance` (`GameplayStatics.GetGameInstance`))))

(event `self.ReceiveActorBeginOverlap`
  (params (OtherActor :type "Actor Object Reference")))

(event `self.Box.OnComponentBeginOverlap`
  (params (OverlappedComponent :type "PrimitiveComponent Object Reference") (OtherActor :type "Actor Object Reference") (OtherComp :type "PrimitiveComponent Object Reference") (OtherBodyIndex :type Integer) (bFromSweep :type Boolean) (SweepResult :type "HitResult Structure (by ref)"))
  ;[1 1 1] Slowing only affects player
  (if (== OtherActor (`GameplayStatics.GetPlayerCharacter` 0))
    (message `/Game/Blueprints/Interfaces/BPI_Player.slowPlayer` OtherActor true)
    (if (not (== (`self.Glue Stick`) "/Game/Audio/SFX/Sc_GlueTrap.Sc_GlueTrap"))
      (bind _returnvalue (`GameplayStatics.CreateSound2D` "/Game/Audio/SFX/Sc_GlueTrap.Sc_GlueTrap" (`/Game/Blueprints/Game/BP_GameInstance.SFX volume` (stale `self.ReceiveBeginPlay` _asbp_game_instance)) 1.0 0.0 null))
      (bind _output_get (set `self.Glue Stick` _returnvalue))
      (`AudioComponent.Play` _output_get 0.0))))

(event `self.Box.OnComponentEndOverlap`
  (params (OverlappedComponent :type "PrimitiveComponent Object Reference") (OtherActor :type "Actor Object Reference") (OtherComp :type "PrimitiveComponent Object Reference") (OtherBodyIndex :type Integer))
  (bind _glue_stick (`self.Glue Stick`))
  ;[1 1 1] Slowing only affects player
  (if (== OtherActor (`GameplayStatics.GetPlayerCharacter` 0))
    (message `/Game/Blueprints/Interfaces/BPI_Player.slowPlayer` OtherActor false)
    (if (`AudioComponent.IsPlaying` _glue_stick)
      (`AudioComponent.Stop` _glue_stick))))

(fn `foodPickup`
  (params (IAvariable :type "Boolean (by ref)"))
  (returns (isPickingUp :type Boolean))
  (return false))

(fn `getAnimOwner`
  (returns (owningCharacter :type "/Game/Blueprints/Player/BP_PlayerCharacterParent Object Reference"))
  (return null))

(fn `getPlayer`
  (returns (PlayerCharacter :type "/Game/Blueprints/Player/BP_MainPlayerCharacter Object Reference"))
  (return null))

(fn `UserConstructionScript`)