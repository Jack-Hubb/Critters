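; BP_CageTrap is a one-shot trap that springs when the player overlaps its Box.
; It moves the Cone component along its vertical axis, then sends each BP_EnemyHuman the Box's world location through CageTrapNotifMessage.
; The cage slam sound plays inside that enemy loop, once per enemy, at the game instance's SFX volume.
; The other functions, such as CageTrapNotif and MouseTrapNotif, are empty stubs.
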(event `self.Box.OnComponentBeginOverlap`
  (params (OverlappedComponent :type "PrimitiveComponent Object Reference") (OtherActor :type "Actor Object Reference") (OtherComp :type "PrimitiveComponent Object Reference") (OtherBodyIndex :type Integer) (bFromSweep :type Boolean) (SweepResult :type "HitResult Structure (by ref)"))
  (bind _cone (`self.Cone`))
  (bind (_relativelocation_x _relativelocation_y) (`KismetMathLibrary.BreakVector` (`SceneComponent.RelativeLocation` _cone)))
  (if (`self.Triggered`)
    _
    (elif (== OtherActor (`GameplayStatics.GetPlayerCharacter` 0))
      (`KismetSystemLibrary.MoveComponentTo` _cone (`KismetMathLibrary.MakeVector` _relativelocation_x _relativelocation_y))
      (set `self.Triggered` true)
      (bind _outactors (`GameplayStatics.GetAllActorsOfClass` "/Game/Blueprints/Enemies/BP_EnemyHuman.BP_EnemyHuman_C"))
      (for _array_element _outactors
        (message `/Game/Blueprints/Interfaces/BPI_Human.CageTrapNotif` _array_element (`SceneComponent.K2_GetComponentLocation` (`self.Box`)))
        (bind _returnvalue (`GameplayStatics.CreateSound2D` "/Game/Audio/SFX/SC_CageSlam.SC_CageSlam" (`/Game/Blueprints/Game/BP_GameInstance.SFX volume` (stale `self.ReceiveBeginPlay` _asbp_game_instance)) 1.0 0.0 null))
        (`AudioComponent.Play` _returnvalue 0.0)))))

(event `self.ReceiveBeginPlay`
  (bind _asbp_game_instance (cast `/Game/Blueprints/Game/BP_GameInstance` (`GameplayStatics.GetGameInstance`))))

(fn `CageTrapNotif`
  (params (Target :type "Vector Structure")))

(fn `foodPickup`
  (params (IAvariable :type "Boolean (by ref)"))
  (returns (isPickingUp :type Boolean))
  (return false))

(fn `getAnimOwner`
  (returns (owningCharacter :type "/Game/Blueprints/Player/BP_PlayerCharacterParent Object Reference"))
  (return null))

(fn `getPlayer`
  (returns (PlayerCharacter :type "/Game/Blueprints/Player/BP_MainPlayerCharacter Object Reference"))
  (return null))

(fn `MouseTrapNotif`
  (params (TargetLocation :type "Vector Structure"))
  (return))

(fn `UserConstructionScript`)