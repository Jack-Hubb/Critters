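; Mouse trap actor that spawns a cheese bait at BeginPlay and springs once when something overlaps its trigger.
; Triggering plays two slash effects, flips the Arrow component and plays a snap sound at the game instance's SFX volume.
; It then stuns player 0, whatever actor overlapped, and sends the trap location to the first BP_EnemyHuman found.
; Its own trap notification functions are empty.
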(event `self.ReceiveBeginPlay`
  (bind (_returnvalue_location _returnvalue_rotation) (`KismetMathLibrary.BreakTransform` (`SceneComponent.K2_GetComponentToWorld` (`self.Arrow3`))))
  (`|SpawnActorFromClass` "/Game/Blueprints/Food/BP_Cheese.BP_Cheese_C" (`KismetMathLibrary.MakeTransform` _returnvalue_location _returnvalue_rotation) "Undefined" "MultiplyWithRoot" null null)
  (bind _asbp_game_instance (cast `/Game/Blueprints/Game/BP_GameInstance` (`GameplayStatics.GetGameInstance`))))

(event `self.w.OnComponentBeginOverlap`
  (params (OverlappedComponent :type "PrimitiveComponent Object Reference") (OtherActor :type "Actor Object Reference") (OtherComp :type "PrimitiveComponent Object Reference") (OtherBodyIndex :type Integer) (bFromSweep :type Boolean) (SweepResult :type "HitResult Structure (by ref)"))
  (if (not (`self.trapTriggered`))
    (`NiagaraFunctionLibrary.SpawnSystemAtLocation` "/Game/Particles/NS_TrapSlash.NS_TrapSlash" (`SceneComponent.K2_GetComponentLocation` (`self.Arrow1`)) (`KismetMathLibrary.MakeRotator` 90.0 -90.0 90.0))
    (`NiagaraFunctionLibrary.SpawnSystemAtLocation` "/Game/Particles/NS_TrapSlash.NS_TrapSlash" (`SceneComponent.K2_GetComponentLocation` (`self.Arrow2`)) (`KismetMathLibrary.MakeRotator` 90.0 -90.0 90.0))
    (`SceneComponent.K2_SetRelativeRotation` (`self.Arrow`) (`KismetMathLibrary.MakeRotator` 180.0) false false)
    (set `self.trapTriggered` true)
    (`GameplayStatics.PlaySound2D` "/Game/Audio/SFX/SC_MouseTrap.SC_MouseTrap" (`/Game/Blueprints/Game/BP_GameInstance.SFX volume` (stale `self.ReceiveBeginPlay` _asbp_game_instance)) 1.0 0.0 null null)
    (message `/Game/Blueprints/Interfaces/BPI_Player.stunnPlayer` (`GameplayStatics.GetPlayerCharacter` 0))
    (bind _outactors (`GameplayStatics.GetAllActorsOfClass` "/Game/Blueprints/Enemies/BP_EnemyHuman.BP_EnemyHuman_C"))
    (for (_array_element _array_index) _outactors
      (if (== _array_index 0)
        (message `/Game/Blueprints/Interfaces/BPI_Human.MouseTrapNotif` _array_element (`SceneComponent.K2_GetComponentLocation` (`self.w`)))))))

(fn `CageTrapNotif`
  (params (Target :type "Vector Structure"))
  (return))

(fn `MouseTrapNotif`
  (params (TargetLocation :type "Vector Structure"))
  (return))

(fn `UserConstructionScript`)