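; Bug enemy that hunts the player, bites for damage, and is destroyed when its health runs out.
; Tick cycles timed searching, rotating and roaming states, with roaming moving forward unless a box trace finds an obstacle.
; Forward box traces that hit the player call Attack, which moves straight ahead or bites on a timer once AttackRange overlaps the player.
; Spawn and hurt sounds scale with the GameInstance SFX volume.
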(event `self.ReceiveBeginPlay`
  (bind _asbp_game_instance (cast `/Game/Blueprints/Game/BP_GameInstance` (`GameplayStatics.GetGameInstance`)))
  (`GameplayStatics.PlaySoundAtLocation` "/Game/Audio/SFX/SC_Bug.SC_Bug" (`self.K2_GetActorLocation`) (struct) (/ (`/Game/Blueprints/Game/BP_GameInstance.SFX volume` _asbp_game_instance) 2.0) 1.0 5.0 null null null null)
  (bind _playercharacter (message `/Game/Blueprints/Interfaces/BPI_Player.getPlayer` (`GameplayStatics.GetPlayerCharacter` 0)))
  (set `self.Player Character` _playercharacter))

(event `Attack`
  (bind _bitetimer (`self.biteTimer`))
  (if (`self.canAttack`)
    (if (>= _bitetimer 1.0)
      (`GameplayStatics.ApplyDamage` (`self.Player Character`) 20.0)
      (set `self.biteTimer` 0.0)
      (else
        (set `self.biteTimer` (+ _bitetimer (stale `self.ReceiveTick` DeltaSeconds)))))
    (else
      (`self.K2_AddActorWorldTransform` (`KismetMathLibrary.MakeTransform` (* (`SceneComponent.GetForwardVector` (`self.FowardArrow`)) 10.0))))))

(event `self.ReceiveTick`
  (params (DeltaSeconds :type "Float (single-precision)"))
  (bind _returnvalue (`self.K2_GetActorLocation`))
  (bind _returnvalue_2 (`self.K2_GetActorLocation`))
  (bind _returnvalue_3 (`self.K2_GetActorLocation`))
  (bind _statetimer (`self.stateTimer`))
  (bind _returnvalue_4 (`SceneComponent.GetForwardVector` (`self.FowardArrow`)))
  (bind _returnvalue_5 (`SceneComponent.GetForwardVector` (`self.FowardArrow`)))
  (bind _returnvalue_6 (`KismetMathLibrary.Conv_VectorToRotator` _returnvalue_4))
  (bind _returnvalue_7 (`KismetMathLibrary.Conv_VectorToRotator` _returnvalue_5))
  (bind _returnvalue_8 (+ _returnvalue (* _returnvalue_4 750.0)))
  (if (<= (`self.Health`) 0.0)
    (`self.K2_DestroyActor`)
    (elif (`self.isSearching`)
      (bind _outhits (`KismetSystemLibrary.BoxTraceMulti` _returnvalue_2 (+ _returnvalue_2 (* _returnvalue_5 1000.0)) (0.0 150.0 50.0) _returnvalue_7 "TraceTypeQuery3" true))
      (for _array_element _outhits
        (if (`GameplayStatics.BreakHitResult` _array_element)
          (if (== (`.HitActor` (`GameplayStatics.BreakHitResult` _array_element)) (`self.Player Character`))
            (`self.Attack` :!label _label))))
      (if (>= _statetimer 3.0)
        (set `self.isSearching` false)
        (set `self.Rotating` true)
        (set `self.stateTimer` 0.0)
        (else
          (set `self.stateTimer` (+ _statetimer DeltaSeconds) :!label _label_2)))
      (elif (`self.Rotating`)
        (`self.K2_AddActorWorldRotation` (struct :`Yaw` 1.0))
        (bind _outhits_2 (`KismetSystemLibrary.BoxTraceMulti` _returnvalue_3 (+ _returnvalue_3 (* _returnvalue_5 750.0)) (0.0 150.0 50.0) _returnvalue_7 "TraceTypeQuery3" true))
        (for _array_element_2 _outhits_2
          (if (`GameplayStatics.BreakHitResult` _array_element_2)
            (if (== (`.HitActor` (`GameplayStatics.BreakHitResult` _array_element_2)) (`self.Player Character`))
              (goto _label))))
        (if (>= (`self.stateTimer`) (`KismetMathLibrary.RandomFloatInRange` 2.0 2.5))
          (set `self.Rotating` false)
          (set `self.Roaming` true)
          (set `self.stateTimer` 0.0)
          (else
            (goto _label_2)))
        (elif (`self.Roaming`)
          (bind _outhit (`KismetSystemLibrary.BoxTraceSingle` (+ (* _returnvalue_4 5.0) _returnvalue) _returnvalue_8 (0.0 150.0 10.0) _returnvalue_6 "TraceTypeQuery1"))
          (if (not (`GameplayStatics.BreakHitResult` _outhit))
            (`self.K2_AddActorWorldTransform` (`KismetMathLibrary.MakeTransform` (* _returnvalue_4 10.0))))
          (bind _outhits_3 (`KismetSystemLibrary.BoxTraceMulti` _returnvalue _returnvalue_8 (0.0 150.0 50.0) _returnvalue_6 "TraceTypeQuery3" true))
          (for _array_element_3 _outhits_3
            (if (`GameplayStatics.BreakHitResult` _array_element_3)
              (if (== (`.HitActor` (`GameplayStatics.BreakHitResult` _array_element_3)) (`self.Player Character`))
                (goto _label))))
          (if (>= (`self.stateTimer`) (`KismetMathLibrary.RandomFloatInRange` 1.0 2.5))
            (set `self.Roaming` false)
            (set `self.isSearching` true)
            (else
              (goto _label_2))))))))

(event `self.attackRange.OnComponentBeginOverlap`
  (params (OverlappedComponent :type "PrimitiveComponent Object Reference") (OtherActor :type "Actor Object Reference") (OtherComp :type "PrimitiveComponent Object Reference") (OtherBodyIndex :type Integer) (bFromSweep :type Boolean) (SweepResult :type "HitResult Structure (by ref)"))
  (if (== OtherActor (`self.Player Character`))
    (set `self.canAttack` true)
    (set `self.stateTimer` 0.0)))

(event `self.attackRange.OnComponentEndOverlap`
  (params (OverlappedComponent :type "PrimitiveComponent Object Reference") (OtherActor :type "Actor Object Reference") (OtherComp :type "PrimitiveComponent Object Reference") (OtherBodyIndex :type Integer))
  (if (== (`self.Player Character`) OtherActor)
    (set `self.canAttack` false)))

(event `self.ReceiveAnyDamage`
  (params (Damage :type "Float (single-precision)") (DamageType :type "DamageType Object Reference") (InstigatedBy :type "Controller Object Reference") (DamageCauser :type "Actor Object Reference"))
  (set `self.health` (- (`self.health`) Damage))
  (`GameplayStatics.PlaySoundAtLocation` "/Game/Audio/SFX/SC_EnemyHurt.SC_EnemyHurt" (`self.K2_GetActorLocation`) (struct) (`/Game/Blueprints/Game/BP_GameInstance.SFX volume` (stale `self.ReceiveBeginPlay` _asbp_game_instance)) 1.0 5.0 null null null null))

(fn `foodPickup`
  (params (IAvariable :type "Boolean (by ref)"))
  (returns (isPickingUp :type Boolean))
  (return false))

(fn `getAnimOwner`
  (returns (owningCharacter :type "/Game/Blueprints/Player/BP_PlayerCharacterParent Object Reference"))
  (return null))

(fn `getPlayer`
  (returns (PlayerCharacter :type "/Game/Blueprints/Player/BP_MainPlayerCharacter Object Reference"))
  (return null))

(fn `UserConstructionScript`)