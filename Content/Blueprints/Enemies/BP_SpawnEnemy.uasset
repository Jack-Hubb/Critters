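; BP_SpawnEnemy is an enemy spawner that periodically creates either a mosquito or a fly.
; Tick accumulates delta time in a timer, and every ten seconds it randomly picks BP_Mosquito or BP_Fly, spawns it, and resets the timer.
; The spawn transform comes from the PlaceholderLocation component's relative transform, so it is used as a world transform without accounting for the spawner's own placement.
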(event `self.ReceiveTick`
  (params (DeltaSeconds :type "Float (single-precision)"))
  (bind _returnvalue (`SceneComponent.GetRelativeTransform` (`self.Placeholder location`)))
  (if (>= (`self.timer`) 10.0)
    (if (`KismetMathLibrary.RandomBool`)
      (`|SpawnActorFromClass` "/Game/Blueprints/Enemies/BP_Mosquito.BP_Mosquito_C" _returnvalue "Undefined" "MultiplyWithRoot" null null)
      (else
        (`|SpawnActorFromClass` "/Game/Blueprints/Enemies/BP_Fly.BP_Fly_C" _returnvalue "Undefined" "MultiplyWithRoot" null null)))
    (set `self.timer` 0.0)
    (else
      (set `self.timer` (+ (`self.timer`) DeltaSeconds)))))

(fn `UserConstructionScript`)