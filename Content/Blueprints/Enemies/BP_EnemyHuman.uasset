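; Human enemy that wanders the level, investigates triggered traps and hunts the player.
; A looping AIMoveTo chain from BeginPlay picks random reachable points, prioritizing mouse trap, then cage trap flags set by notification events.
; Tick runs a timed forward box trace, chasing a detected player or dealing one-time damage up close.
; Reaching a cage trap with the player nearby loads the hub level.
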(event `/Game/Blueprints/Interfaces/BPI_Human.CageTrapNotif`
  (params (Target :type "Vector Structure"))
  (set `self.cageTrapTriggered` true))

(event `/Game/Blueprints/Interfaces/BPI_Human.MouseTrapNotif`
  (params (TargetLocation :type "Vector Structure"))
  (set `self.mouseTrapTriggered` true))

(event `self.ReceiveBeginPlay`
  (bind _randomlocation (`NavigationSystemV1.K2_GetRandomReachablePointInRadius` (`self.K2_GetActorLocation`) 2000.0 null null))
  (set `self.god` true)
  (if (`self.mouseTrapTriggered`) :!label _label
    (set `self.walking` true)
    (`|AIMoveTo` self (stale `/Game/Blueprints/Interfaces/BPI_Human.MouseTrapNotif` TargetLocation) null 300.0 :!label _label_2
      (:`then`
        (`/Engine/EditorBlueprintResources/StandardMacros.DoOnce` false
          (:`Completed`
            (`GameplayStatics.PlaySoundAtLocation` null (0.0 0.0 0.0) (struct) 1.0 1.0 0.0 null null null null))))
      (:`OnSuccess`
        (set `self.mouseTrapTriggered` false)
        (goto _label)))
    (elif (`self.cageTrapTriggered`)
      (set `self.walking` true)
      (`|AIMoveTo` self (stale `/Game/Blueprints/Interfaces/BPI_Human.CageTrapNotif` Target) null 300.0
        (:`then`
          (`/Engine/EditorBlueprintResources/StandardMacros.DoOnce` false
            (:`Completed`
              (`GameplayStatics.PlaySoundAtLocation` null (0.0 0.0 0.0) (struct) 1.0 1.0 0.0 null null null null))))
        (:`OnSuccess`
          (if (<= (`KismetMathLibrary.Vector_Distance` (`self.K2_GetActorLocation` (`GameplayStatics.GetPlayerCharacter` 0)) (`self.K2_GetActorLocation`)) 100.0)
            (`/Engine/EditorBlueprintResources/StandardMacros.DoOnce` false
              (:`Completed`
                (`GameplayStatics.PlaySoundAtLocation` (`self.Sound_0`) (0.0 0.0 0.0) (struct) 1.0 1.0 0.0 null null null null)
                (`GameplayStatics.OpenLevelBySoftObjectPtr` "/Game/Maps/L_Hub.L_Hub"))))
          (set `self.cageTrapTriggered` false)
          (goto _label)))
      (else
        (set `self.walking` true)
        (`|AIMoveTo` self (`KismetMathLibrary.MakeVector` (.x _randomlocation) (.y _randomlocation) (.z _randomlocation)) null 100.0
          (:`then`
            (`/Engine/EditorBlueprintResources/StandardMacros.DoOnce` false
              (:`Completed`
                (`GameplayStatics.PlaySoundAtLocation` (`self.walkSound`) (`self.K2_GetActorLocation`) (struct) 1.0 1.0 0.0 null null null null))))
          (:`OnSuccess`
            (if (`self.mouseTrapTriggered`)
              (goto _label_2)
              (elif (`self.cageTrapTriggered`)
                (set `self.walking` false)
                (goto _label)
                (else
                  (`KismetSystemLibrary.Delay` (`KismetMathLibrary.RandomFloatInRange` 2.0 4.0))
                  (goto _label))))))))))

(event `self.ReceiveTick`
  (params (DeltaSeconds :type "Float (single-precision)"))
  (bind _returnvalue (`self.K2_GetActorLocation`))
  (bind _returnvalue_2 (`SceneComponent.GetForwardVector` (`self.Arrow1`)))
  (`parent.ReceiveTick` DeltaSeconds)
  (set `self.curTimer` (+ DeltaSeconds (`self.curTimer`)))
  (if (>= (`self.curTimer`) (`self.MaxTimer`))
    (bind _outhits (`KismetSystemLibrary.BoxTraceMulti` _returnvalue (+ _returnvalue (* _returnvalue_2 1000.0)) (200.0 1000.0 500.0) (`KismetMathLibrary.Conv_VectorToRotator` _returnvalue_2) "TraceTypeQuery3"))
    (set `self.curTimer` 0.0)
    (for _array_element _outhits
      (if (== (`.HitActor` (`GameplayStatics.BreakHitResult` _array_element)) (`GameplayStatics.GetPlayerCharacter` 0))
        (if (<= (`.Distance` (`GameplayStatics.BreakHitResult` _array_element)) 100.0)
          (`/Engine/EditorBlueprintResources/StandardMacros.DoOnce` false
            (:`Completed`
              (`GameplayStatics.PlaySoundAtLocation` (`self.Sound_0`) (`self.K2_GetActorLocation`) (struct) 1.0 1.0 0.0 null null null null)
              (`GameplayStatics.ApplyDamage` (`.HitActor` (`GameplayStatics.BreakHitResult` _array_element)) 100.0)
              (goto _label)))
          (else
            (bind (_returnvalue_x _returnvalue_y) (`KismetMathLibrary.BreakVector` (`self.K2_GetActorLocation` (`.HitActor` (`GameplayStatics.BreakHitResult` _array_element)))))
            (`|AIMoveTo` self (`KismetMathLibrary.MakeVector` _returnvalue_x _returnvalue_y) null 15.0
              (:`OnSuccess`
                (goto _label)))))))))

(fn `UserConstructionScript`
  (`parent.UserConstructionScript`))