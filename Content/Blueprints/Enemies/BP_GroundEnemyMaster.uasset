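; Master ground enemy Blueprint that wanders the navmesh and handles its own damage and death.
; From BeginPlay it moves to random reachable points around itself, pausing briefly after each success; a failed move ends the loop.
; AnyDamage sets Health to Damage minus Health, an inverted subtraction.
; Tick destroys the actor when God is off and Health is at or below MaxHealth, rather than zero.
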(event `self.ReceiveBeginPlay`
  (bind _randomlocation (`NavigationSystemV1.K2_GetRandomReachablePointInRadius` (`self.K2_GetActorLocation`) 1000.0 null null))
  (`|AIMoveTo` self (`KismetMathLibrary.MakeVector` (.x _randomlocation) (.y _randomlocation) (.z _randomlocation)) null 100.0 :!label _label
    (:`OnSuccess`
      (`KismetSystemLibrary.Delay` (`KismetMathLibrary.RandomFloatInRange` 2.0 4.0))
      (goto _label))))

(event `self.ReceiveTick`
  (params (DeltaSeconds :type "Float (single-precision)"))
  ;[1 1 1] death condition
  (if (`self.god`)
    _
    (elif (<= (`self.health`) (`self.maxHealth`))
      (`self.K2_DestroyActor`))))

(event `self.ReceiveAnyDamage`
  (params (Damage :type "Float (single-precision)") (DamageType :type "DamageType Object Reference") (InstigatedBy :type "Controller Object Reference") (DamageCauser :type "Actor Object Reference"))
  ;[1 1 1] Damage Input
  (set `self.health` (- Damage (`self.health`))))

(fn `UserConstructionScript`)