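; Base Blueprint for flying enemies, handling movement setup, damage and death.
; BeginPlay adds a BPC_FindMoveToVector component to the actor.
; AnyDamage sets Health to the incoming damage minus current Health, rather than subtracting damage from Health.
; Tick destroys the actor whenever Health is less than or equal to MaxHealth, rather than checking against zero.
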(event `self.ReceiveBeginPlay`
  (`AddComponent|NODE_AddBPC_FindMoveToVector-0` :`owner` self))

(event `self.ReceiveTick`
  (params (DeltaSeconds :type "Float (single-precision)"))
  ;[1 1 1] death condition
  (if (<= (`self.health`) (`self.maxHealth`))
    (`self.K2_DestroyActor`)))

(event `self.ReceiveAnyDamage`
  (params (Damage :type "Float (single-precision)") (DamageType :type "DamageType Object Reference") (InstigatedBy :type "Controller Object Reference") (DamageCauser :type "Actor Object Reference"))
  ;[1 1 1] Recieved Damage
  (set `self.health` (- Damage (`self.health`))))

(fn `UserConstructionScript`)