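; Claw attack component that gives its owner a melee swipe when the IA_Claw input completes.
; A forward box trace on the Visibility channel damages every hit actor, scaling damage by the input's elapsed time, capped at one second.
; It then spawns a slash Niagara effect and plays an attack sound at the game instance's SFX volume.
; The owner's Swiping flag is set at the start and cleared after a short delay.
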(event `EnhancedInput|/Game/Blueprints/Game/Input/Actions/IA_Claw`
  (params (ActionValue :type Boolean) (ElapsedSeconds :type "Float (double-precision)") (TriggeredSeconds :type "Float (double-precision)") (InputAction :type "InputAction Object Reference" :default "/Game/Blueprints/Game/Input/Actions/IA_Claw.IA_Claw"))
  (bind _owner (`self.owner`))
  (bind _owner_2 (`self.owner`))
  (bind _returnvalue (`Actor.GetActorForwardVector` _owner))
  (bind _returnvalue_2 (`Actor.K2_GetActorLocation` _owner_2))
  (bind _returnvalue_3 (`SceneComponent.GetForwardVector` (`Actor.RootComponent` _owner_2)))
  (:`Completed`
    (set `/Game/Blueprints/Player/BP_PlayerCharacterParent.swiping` true (`self.owner`))
    (bind _asbp_game_instance (cast `/Game/Blueprints/Game/BP_GameInstance` (`GameplayStatics.GetGameInstance`)))
    ;[1 1 1] Locate Enemies in Box
    (bind _outhits (`KismetSystemLibrary.BoxTraceMulti` _returnvalue_2 (+ _returnvalue_2 (* _returnvalue_3 225.0)) (50.0 150.0 30.0) (`KismetMathLibrary.Conv_VectorToRotator` _returnvalue_3) "TraceTypeQuery1"))
    ;[1 1 1] Damage Enemies
    (for _array_element _outhits
      (bind _returnvalue_4 (`GameplayStatics.ApplyDamage` (`.HitActor` (`GameplayStatics.BreakHitResult` _array_element)) (* 10.0 (`KismetMathLibrary.FClamp` ElapsedSeconds)))))
    ;[1 1 1] Spawn Particle System
    (`NiagaraFunctionLibrary.SpawnSystemAtLocation` "/Game/Particles/NS_Slash.NS_Slash" (+ (* 50.0 _returnvalue) (`Actor.K2_GetActorLocation` _owner)) (`KismetMathLibrary.Conv_VectorToRotator` (`KismetMathLibrary.GreaterGreater_VectorRotator` (* _returnvalue -1.0) (struct :`Yaw` 45.0))))
    (`GameplayStatics.PlaySound2D` "/Game/Audio/SFX/SC_PlayerAttack.SC_PlayerAttack" (`/Game/Blueprints/Game/BP_GameInstance.SFX volume` _asbp_game_instance) 1.0 0.0 null null)
    (`KismetSystemLibrary.Delay` 2.0)
    (set `/Game/Blueprints/Player/BP_PlayerCharacterParent.swiping` false (`self.owner`))))