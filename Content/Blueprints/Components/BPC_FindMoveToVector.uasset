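; Actor component that makes its owner wander by periodically turning to a random rotation and gliding to a random point.
; Tick uses a DoOnce to set a looping Move timer, and each Move resets that gate.
; Move eases the root component to forward-vector X/Y offsets with random height, without adding the current location.
; FindMove is empty, with an unconnected lerp-based movement draft left in its graph.
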(event `self.ReceiveTick`
  (params (DeltaSeconds :type "Float (single-precision)"))
  (`/Engine/EditorBlueprintResources/StandardMacros.DoOnce` false :!label _label
    (:`Completed`
      (`KismetSystemLibrary.K2_SetTimerDelegate` (delegate `Move`) 3.0 true))))

(event `Move`
  (bind _owner (`self.owner`))
  (bind (_returnvalue_x _returnvalue_y) (`KismetMathLibrary.BreakVector` (* (`KismetMathLibrary.GetForwardVector` (`Actor.K2_GetActorRotation` _owner)) (`KismetMathLibrary.RandomFloatInRange` 100.0 500.0))))
  (`Actor.K2_SetActorRotation` _owner (`KismetMathLibrary.MakeRotator` (`KismetMathLibrary.RandomFloatInRange` 0.0 360.0) (`KismetMathLibrary.RandomFloatInRange` 0.0 360.0) (`KismetMathLibrary.RandomFloatInRange` 0.0 360.0)) false)
  (`KismetSystemLibrary.MoveComponentTo` (`Actor.RootComponent` (`self.owner`)) (`KismetMathLibrary.MakeVector` _returnvalue_x _returnvalue_y (`KismetMathLibrary.RandomFloatInRange` 10.0 500.0)) (struct) true true 2.0)
  (goto _label :!via `Reset`))

(fn `Find Move`
  (params (DeltaTime :type "Float (double-precision)")))